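; Enemy melee attack ability that turns the avatar toward its combat target and plays a random tagged attack montage.
; The montage's gameplay event triggers a sphere check at the tagged combat socket for live players, with a debug sphere drawn.
; Non-friendly hits take damage and spawn their own blood effect.
; Any hit fires one MeleeImpact GameplayCue carrying the montage tag, and the ability ends after the check or montage end.
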(event Ability|EventActivateAbility
  (bind _returnvalue (Ability|GetAvatarActorfromActorInfo))
  (bind _returnvalue_2 (Ability|GetAvatarActorfromActorInfo))
  (bind _returnvalue_3 (Ability|GetAvatarActorfromActorInfo))
  (bind _returnvalue_4 (Class|EnemyInterface|GetCombatTarget(Message) _returnvalue_3))
  (bind _ascombat_interface (Utilities|Casting|CastToCombatInterface _returnvalue_3))
  (Class|CombatInterface|UpdateFacingTarget _ascombat_interface (Transformation|GetActorLocation _returnvalue_4))
  (bind _returnvalue_5 (Class|CombatInterface|GetAttackMontages(Message) (Ability|GetAvatarActorfromActorInfo)))
  (bind _output_get (Variables|Default|SetTaggedMontage (Class|AuraDamageGameplayAbility|GetRandomTaggedMontagefromArray _returnvalue_5)))
  (|PlayMontageandWaitProxy "None" (.Montage (Utilities|Struct|BreakTaggedMontage _output_get)) 1.0 "None" false 1.0 0.0 false
    (:then
      (Ability|Tasks|WaitGameplayEvent (.MontageTag (Utilities|Struct|BreakTaggedMontage _output_get)) 0
        (:EventReceived
          (bind _returnvalue_6 (Class|CombatInterface|GetCombatSocketLocation(Message) _returnvalue_2 (.SocketTag (Utilities|Struct|BreakTaggedMontage _output_get))))
          (Variables|Default|SetCombatSocketLocation _returnvalue_6)
          (bind _outoverlappingactors (Class|AuraAbilitySystemLibrary|GetLivePlayerswithRadius _returnvalue_2 (Utilities|Array|MakeArray _returnvalue_2) 45.0 (Variables|Default|GetCombatSocketLocation)))
          (Rendering|Debug|DrawDebugSphere (Variables|Default|GetCombatSocketLocation) 45.0 12 "(R=1.000000,G=0.000000,B=0.216577,A=1.000000)" 1.0)
          (for _array_element _outoverlappingactors
            (if (Class|AuraAbilitySystemLibrary|IsNotFriend (Ability|GetAvatarActorfromActorInfo) _array_element)
              (Class|AuraDamageGameplayAbility|CauseDamage _array_element)
              (Variables|Default|SetHasHitTarget true)
              (bind _returnvalue_7 (Class|CombatInterface|GetBloodEffect(Message) _array_element))
              (Niagara|SpawnSystematLocation _returnvalue_7 (Variables|Default|GetCombatSocketLocation))))
          (if (Variables|Default|GetHasHitTarget)
            ;[1 1 1] 将一些必要的信息传入GameplayCue里面
            (bind _returnvalue_8 (Class|EnemyInterface|GetCombatTarget(Message) _returnvalue))
            (Class|GameplayAbility|ExecuteGameplayCuewithParams "(TagName=\"GameplayCue.MeleeImpact\")" (Ability|GameplayCue|MakeGameplayCueParameters :AggregatedSourceTags (GameplayTags|MakeGameplayTagContainerfromTag (.MontageTag (Utilities|Struct|BreakTaggedMontage (Variables|Default|GetTaggedMontage)))) :Location (Variables|Default|GetCombatSocketLocation) :EffectCauser _returnvalue :SourceObject _returnvalue_8)))
          (Ability|EndAbility))))
    (:OnCompleted
      (Ability|EndAbility :!label _label))
    (:OnInterrupted
      (goto _label))
    (:OnCancelled
      (goto _label))))

(event Ability|EventOnEndAbility
  (params (bWasCancelled :type Boolean)))