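; BP_FireBalls is the fireball actor for Aura's FireBlast skill, flying out and returning like a boomerang before exploding.
; On authority, StarOutgoingTimeline lerps it from its start to an apex at a set distance along its forward vector.
; It then clears its ignore list, and ReturningTimeline homes it on ReturnActor's live location.
; Within explosion distance of ReturnActor, it calls OnHit and destroys itself.
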(event EventStarOutgoingTimeline
  (Networking|SwitchHasAuthority
    (:Authority
      (CallFunction|计算初始位置和终点位置)
      (bind _outgoingtrack (Timeline|OutGoingTimeline Play)
        (:Update
          (Transformation|SetActorLocation (Math|Vector|Lerp(Vector) (Variables|Default|Get初始位置) (Variables|Default|Get顶点的位置) _outgoingtrack) false false))
        (:Finished
          (Class|AuraFireBall|EmptyIgnoreList)
          (bind _return (Timeline|ReturningTimeline Play)
            (:Update
              (Transformation|SetActorLocation (Math|Vector|Lerp(Vector) (Variables|Default|Get顶点的位置) (Transformation|GetActorLocation (Variables|Default|GetReturnActor)) _return) false false)
              (if (CallFunction|是否处在爆炸距离内)
                (Class|AuraProjectile|OnHit)
                (Actor|DestroyActor)))))))))

(fn ConstructionScript)

(fn 计算初始位置和终点位置
  (Variables|Default|Set初始位置 (Transformation|GetActorLocation))
  (Variables|Default|Set顶点的位置 (+ (Variables|Default|Get初始位置) (* (Transformation|GetActorForwardVector) (Variables|Default|Get飞行距离)))))

(fn 是否处在爆炸距离内
  (return (<= (Math|Vector|VectorLength (- (Transformation|GetActorLocation) (Transformation|GetActorLocation (Variables|Default|GetReturnActor)))) (Variables|Default|Get爆炸距离))))