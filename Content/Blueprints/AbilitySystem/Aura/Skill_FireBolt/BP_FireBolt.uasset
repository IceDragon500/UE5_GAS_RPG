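; BP_FireBolt is the Fire Bolt skill's projectile Blueprint, with a Tick fallback for bolts whose homing target disappears mid-flight.
; Tick measures the distance between the current location and a stored LastFrame position, treating a value below MinDisttance as a stalled bolt.
; It then plays the impact sound, spawns the fire explosion effect and destroys the actor.
; As shown, LastFrame is only assigned to itself, never updated from the current location.
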(event EventBeginPlay)

(event Collision|EventActorBeginOverlap
  (params (OtherActor :type Actor%20Object%20Reference)))

(event EventTick
  (params (DeltaSeconds :type Float%20%28single-precision%29))
  ;[1 1 1] 334课
  ; 解决了火球在飞行过程中，如果目标消失，火球飞行到目标地点不会消失的问题
  (Variables|Default|SetLastFrame (Variables|Default|GetLastFrame))
  (Variables|Default|SetNewFrame (Transformation|GetActorLocation))
  (if (< (Math|Vector|VectorLength (- (Variables|Default|GetNewFrame) (Variables|Default|GetLastFrame))) (Variables|Default|GetMinDisttance))
    (Audio|SpawnSoundatLocation "/Game/Assets/Sounds/Abilities/FireBolt/sfx_FireBolt_Impact.sfx_FireBolt_Impact" (Variables|Default|GetNewFrame) "0, 0, 0" 1.0 1.0 0.0 0 0)
    (Niagara|SpawnSystematLocation "/Game/Assets/Effects/Projectiles/FireExplosion/NS_FireExplosion.NS_FireExplosion" (Variables|Default|GetNewFrame))
    (Actor|DestroyActor)))

(fn ConstructionScript)