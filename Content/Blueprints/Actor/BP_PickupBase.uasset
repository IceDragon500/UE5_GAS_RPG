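; BP_PickupBase is a base pickup actor that animates items popping out, named in the timeline as monster drops.
; On BeginPlay, a timeline drives a vertical hop scaled by SpawnApex above InitialLocation, plus a uniform scale curve.
; When it finishes, it calls StartSinusoidalMovement and StartRotation, whose logic lives outside this graph.
; Tick applies CalculatedLocation and CalculatedRotation to the actor every frame, without sweeping.
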(event EventBeginPlay
  (bind (_direction _怪物爆道具的跳跃效果 _怪物爆道具的放大缩小) (Timeline|PickupTimeline Play)
    (:Update
      (CallFunction|爆道具的跳跃效果 _怪物爆道具的跳跃效果)
      (Transformation|SetActorScale3D (Math|Vector|MakeVector _怪物爆道具的放大缩小 _怪物爆道具的放大缩小 _怪物爆道具的放大缩小)))
    (:Finished
      (Class|AuraEffectActor|StartSinusoidalMovement)
      (Class|AuraEffectActor|StartRotation))))

(event Collision|EventActorBeginOverlap
  (params (OtherActor :type Actor%20Object%20Reference)))

(event EventTick
  (params (DeltaSeconds :type Float%20%28single-precision%29))
  (Transformation|SetActorLocation (Variables|Default|GetCalculatedLocation) false false)
  (Transformation|SetActorRotation (Variables|Default|GetCalculatedRotation)))

(fn ConstructionScript)

(fn 爆道具的跳跃效果
  (params (A :type Float%20%28double-precision%29))
  (bind _initiallocation (Variables|Default|GetInitialLocation))
  (bind (_x _y _z) (Math|Vector|BreakVector _initiallocation))
  (Variables|Default|SetCalculatedLocation (Math|Vector|MakeVector _x _y (+ _z (* A (Variables|Default|GetSpawnApex))))))