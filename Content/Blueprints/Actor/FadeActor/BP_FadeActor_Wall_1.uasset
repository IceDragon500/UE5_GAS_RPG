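; Wall actor that fades its mesh out and back in, running FadeOut at BeginPlay and FadeIn after a short delay.
; Construction caches the original materials and builds dynamic instances from FadeMaterialInstance.
; FadeOut swaps in those instances and plays a timeline driving their "Fade" parameter, which FadeIn reverses.
; When the timeline finishes with Fade at half or above, the original materials are restored.
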(event EventBeginPlay
  (CallFunction|FadeOut)
  (Utilities|FlowControl|Delay 2.0)
  (CallFunction|Fadein))

(event EventFadeOut
  (CallFunction|SetmaterialstoDynamicInstances)
  (bind _fade (Timeline|FadeTimeline Play)
    (:Update
      (for _array_element (Variables|Default|GetDynamicMaterialInstances)
        (Rendering|Material|SetScalarParameterValue _array_element "Fade" _fade :!class /Script/Engine.MaterialInstanceDynamic)))
    (:Finished
      (if (>= _fade 0.5)
        (for (_array_element_2 _array_index) (Variables|Default|GetOriginalMaterials)
          (Rendering|Material|SetMaterial (Variables|Default|GetMesh) _array_index _array_element_2))
        (elif (<= _fade 0.2)
          _)))))

(event EventFadein
  (bind _fade (Timeline|FadeTimeline Reverse)
    (:Update
      (for _array_element (Variables|Default|GetDynamicMaterialInstances)
        (Rendering|Material|SetScalarParameterValue _array_element "Fade" _fade :!class /Script/Engine.MaterialInstanceDynamic)))
    (:Finished
      (if (>= _fade 0.5)
        (for (_array_element_2 _array_index) (Variables|Default|GetOriginalMaterials)
          (Rendering|Material|SetMaterial (Variables|Default|GetMesh) _array_index _array_element_2))
        (elif (<= _fade 0.2)
          _)))))

(fn ConstructionScript
  (Utilities|Array|Clear (Variables|Default|GetDynamicMaterialInstances))
  (Variables|Default|SetOriginalMaterials (Rendering|Material|GetMaterials (Variables|Default|GetMesh)))
  (for _array_element (Variables|Default|GetFadeMaterialInstance)
    (bind _returnvalue (Rendering|Material|CreateDynamicMaterialInstance _array_element "None" "None" :!class /Script/Engine.KismetMaterialLibrary))
    (Utilities|Array|AddUnique (Variables|Default|GetDynamicMaterialInstances) _returnvalue)))

(fn SetmaterialstoDynamicInstances
  (for (_array_element _array_index) (Variables|Default|GetDynamicMaterialInstances)
    (Rendering|Material|SetMaterial (Variables|Default|GetMesh) _array_index _array_element)))