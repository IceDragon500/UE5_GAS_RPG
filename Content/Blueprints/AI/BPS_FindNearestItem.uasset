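; Behavior tree service that, on each AI tick, is meant to find the nearest item to the controlled pawn.
; It gathers AuraEffectActors tagged "Item" and measures each one's distance to the pawn.
; The closer-than comparison is left unconnected, so the last valid actor is picked rather than the nearest.
; The pick is only shown as a timed red debug line, with no blackboard write.
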(event EventReceiveTickAI
  (params (OwnerController :type AI%20Controller%20Object%20Reference) (ControlledPawn :type Pawn%20Object%20Reference) (DeltaSeconds :type Float%20%28single-precision%29))
  (CallFunction|找到最近的道具 ControlledPawn))

(fn 找到最近的道具
  (params (ControlledPawn :type Pawn%20Object%20Reference))
  (Variables|Default|Set距离最近的Actor 0)
  (Variables|Default|Set最近的距离 999999999.0)
  (bind _outactors (Actor|GetAllActorsOfClasswithTag "/Script/Aura.AuraEffectActor" "Item"))
  (for _array_element _outactors
    (bind _output_get (Variables|Default|Set被找到的Actor _array_element))
    (Utilities|IsValid _output_get
      (:Is%20Valid
        (Utilities|IsValid ControlledPawn
          (:Is%20Valid
            (bind _output_get_2 (Variables|Default|Set检测到的距离 (Transformation|GetDistanceTo ControlledPawn (Variables|Default|Get被找到的Actor))))
            (if true
              (Variables|Default|Set最近的距离 (Variables|Default|Get检测到的距离))
              (Variables|Default|Set距离最近的Actor (Variables|Default|Get被找到的Actor))))))))
  (Rendering|Debug|DrawDebugLine (Transformation|GetActorLocation ControlledPawn) (Transformation|GetActorLocation (Variables|Default|Get距离最近的Actor)) "(R=1.000000,G=0.000000,B=0.000000,A=1.000000)" 4.0 0.0))