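; Behavior tree service that finds the nearest opposing actor for an AI pawn to target, despite its player-specific name.
; Each AI tick, it sets the target tag to Enemy for Player-tagged pawns and to Player for all others.
; It then linearly scans all actors with that tag for the closest one.
; The resulting actor and its distance are written to Blackboard keys through selectors.
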(event EventReceiveTickAI
  (params (OwnerController :type AI%20Controller%20Object%20Reference) (ControlledPawn :type Pawn%20Object%20Reference) (DeltaSeconds :type Float%20%28single-precision%29))
  (CallFunction|SetTargetTag ControlledPawn)
  (CallFunction|FindNearestPlayer ControlledPawn))

(fn SetTargetTag
  (params (ControllerPawn :type Actor%20Object%20Reference))
  ;[1 1 1] 这里的意思是：
  ; 我们从ControllerPawn上获取Tag
  ; 如果这个Tag是Player，则我们设置TargetTag为Enemy 就是设置目标是敌人
  ; 如果不是Player，因为我们现在只设置了Player和Enemy，所以ControlledPawn就是Enemy
  ; 目标自然就是Player
  (if (Actor|ActorHasTag ControllerPawn "Player")
    (Variables|Default|SetTargetTag "Enemy")
    (else
      (Variables|Default|SetTargetTag "Player"))))

(fn FindNearestPlayer
  (params (ControlledPawn :type Pawn%20Object%20Reference))
  (LocalVariables|SetClosestActor 0)
  (LocalVariables|SetClosesDistance 9999999999.0)
  (bind _outactors (Actor|GetAllActorswithTag (Variables|Default|GetTargetTag)))
  (for _array_element _outactors
    (bind _output_get (LocalVariables|SetActor _array_element))
    (Utilities|IsValid _output_get
      (:Is%20Valid
        ;[1 1 1] 获取Ai与找到Actor的距离
        (Utilities|IsValid ControlledPawn
          (:Is%20Valid
            ;[1 1 1] 检查获取到的距离Calculated和Closes这两个距离谁更小
            ; 如果Calculated更小，则设置Closes为Calculated
            ; 并设置Actor为当前找到的这个Actor
            (bind _output_get_2 (LocalVariables|SetCalculatedDistance (Transformation|GetDistanceTo ControlledPawn (LocalVariables|GetActor))))
            (if (< _output_get_2 (LocalVariables|GetClosesDistance))
              (LocalVariables|SetClosesDistance (LocalVariables|GetCalculatedDistance))
              (LocalVariables|SetClosestActor (LocalVariables|GetActor))))))))
  (Class|BTFunctionLibrary|SetBlackboardValueasObject (Variables|Default|GetTargetToFollow_Selector) (LocalVariables|GetClosestActor))
  (Class|BTFunctionLibrary|SetBlackboardValueasFloat (Variables|Default|GetDistanceToTarget_Selector) (LocalVariables|GetClosesDistance)))