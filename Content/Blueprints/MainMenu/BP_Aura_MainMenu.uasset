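; Main menu scene actor that plays the menu music and shows the menu widget over a cine camera view.
; On BeginPlay it creates WBP_MainMenu, switches the view target to the level's CineCameraActor and sets UI-only input with a visible cursor.
; Each Tick advances a timer that resets past two pi, bobbing the FireBall vertically around its starting location with an amplitude-scaled sine.
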(event EventBeginPlay
  (bind _returnvalue (Game|GetPlayerController 0))
  (Variables|Default|SetFireBallLocation (Transformation|GetWorldLocation (Variables|Default|GetFireBall)))
  (Audio|PlaySound2D "/Game/Assets/Sounds/Music/Music_MainMenu.Music_MainMenu" 1.0 1.0 0.0 0 0)
  (bind _returnvalue_2 (UserInterface|CreateWidget "/Game/Blueprints/UI/MainMenu/WBP_MainMenu.WBP_MainMenu_C"))
  (Variables|Default|SetMainMenuWidget _returnvalue_2)
  (UserInterface|Viewport|AddtoViewport _returnvalue_2 0)
  (bind _returnvalue_3 (Actor|GetActorOfClass "/Script/CinematicCamera.CineCameraActor"))
  (Game|Player|SetViewTargetwithBlend _returnvalue _returnvalue_3 0.0 "VTBlend_Linear" 0.0 false)
  (Input|SetInputModeUIOnly _returnvalue (Variables|Default|GetMainMenuWidget) "DoNotLock" false)
  (Variables|/Script/Engine.PlayerController|SetbShowMouseCursor _returnvalue true))

(event EventTick
  (params (DeltaSeconds :type Float%20%28single-precision%29))
  (CallFunction|更新时间 DeltaSeconds)
  (Transformation|SetWorldLocation (Variables|Default|GetFireBall) (+ (Variables|Default|GetFireBallLocation) (Math|Vector|MakeVector 0.0 0.0 (CallFunction|SinTime))) false false))

(fn ConstructionScript)

(fn 更新时间
  (params (A :type Float%20%28double-precision%29))
  (bind _output_get (Variables|Default|Set时间 (+ A (Variables|Default|Get时间))))
  (if (> _output_get 6.28318)
    (Variables|Default|Set时间 0.0)))

(fn SinTime
  (return (* (Math|Trig|Sin(Radians) (Variables|Default|Get时间)) (Variables|Default|Get振幅缩放))))