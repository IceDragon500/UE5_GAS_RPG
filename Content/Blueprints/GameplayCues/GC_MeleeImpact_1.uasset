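; Gameplay cue for melee hits that plays an impact sound and spawns a blood effect at the hit location.
; OnExecute uses an aggregated source tag to ask the effect causer for its tagged montage, which supplies the impact sound.
; The blood particle system also comes from the effect causer through a message call.
; The parent OnExecute is returned inside the tag loop, so only the first tag is handled.
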(fn OnExecute
  (params (MyTarget :type Actor%20Object%20Reference) (Parameters :type Gameplay%20Cue%20Parameters%20Structure%20%28by%20ref%29))
  (bind (_normalizedmagnitude _rawmagnitude _effectcontext _matchedtagname _originaltag _aggregatedsourcetags _aggregatedtargettags _location _normal _instigator _effectcauser _sourceobject) (Ability|GameplayCue|BreakGameplayCueParameters Parameters))
  (LocalVariables|SetLocation _location)
  (LocalVariables|SetEffectCauser _effectcauser)
  (LocalVariables|SetSourceObject _sourceobject)
  (for _array_element (GameplayTags|BreakGameplayTagContainer _aggregatedsourcetags)
    (bind _returnvalue (Class|CombatInterface|GetTaggedMontagebyTag(Message) (LocalVariables|GetEffectCauser) _array_element))
    (Audio|PlaySoundatLocation (LocalVariables|GetEffectCauser) (.ImpactSound (Utilities|Struct|BreakTaggedMontage _returnvalue)) (LocalVariables|GetLocation) "0, 0, 0" 1.0 1.0 0.0 0 0 0 0)
    (bind _returnvalue_2 (Class|CombatInterface|GetBloodEffect(Message) (LocalVariables|GetEffectCauser)))
    (Niagara|SpawnSystematLocation (LocalVariables|GetEffectCauser) _returnvalue_2 (LocalVariables|GetLocation))
    (return (|CallParentFunction MyTarget Parameters))))